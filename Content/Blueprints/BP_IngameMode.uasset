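; BP_IngameMode is the in-game mode Blueprint that handles score rewards and dispatches victory.
; Enemy hit and kill events cast the offender to BP_IngamePlayerPawn, add the matching reward through RewardPlayer, then pass the new score to BP_GameInstance's UpdateHighScore.
; The game instance reference is cached on BeginPlay.
; When all enemies are killed, it calls ChangeTheGameMode to switch to the victory state.
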(event EventOnAllEnemiesKilled
  ;[1 1 1] Dispatch Victory
  (Utilities|ChangetheGameMode "NewEnumerator2"))

(event EventBeginPlay
  ;[1 1 1] Init Variables
  (bind _asbp_game_instance (Utilities|Casting|CastToBP_GameInstance (Game|GetGameInstance)))
  (Variables|Gameplay|SetGameInstanceRef _asbp_game_instance))

(event EventOnEnemyHit
  (params (Target :type Enemy%20Object%20Reference) (Ofender :type Player%20Pawn%20Object%20Reference))
  ;[1 1 1] Enemy Score Rewards
  (bind _asbp_ingame_player_pawn (Utilities|Casting|CastToBP_IngamePlayerPawn Ofender))
  (bind _newscore (CallFunction|RewardPlayer _asbp_ingame_player_pawn (Variables|Rewards|GetHitReward)))
  (Default|UpdateHighScore (Variables|Gameplay|GetGameInstanceRef) _newscore))

(event EventOnEnemyKilled
  (params (Target :type Enemy%20Object%20Reference) (Ofender :type Player%20Pawn%20Object%20Reference))
  ;[1 1 1] Enemy Score Rewards
  (bind _asbp_ingame_player_pawn (Utilities|Casting|CastToBP_IngamePlayerPawn Ofender))
  (bind _newscore (CallFunction|RewardPlayer _asbp_ingame_player_pawn (Variables|Rewards|GetKillReward)))
  (Default|UpdateHighScore (Variables|Gameplay|GetGameInstanceRef) _newscore))

(fn ConstructionScript)

(fn RewardPlayer
  (params (Player :type BP%20Ingame%20Player%20Pawn%20Object%20Reference) (Reward :type Integer))
  (bind _output_get (LocalVariables|SetOutNewScore (+ (Default|GetScore Player) Reward)))
  (Default|SetScore Player _output_get)
  (return (LocalVariables|GetOutNewScore)))