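; BP_PostgamePlayerPawn is the player pawn for the postgame, presenting the victory menu.
; On BeginPlay it switches to UI-only input with a visible cursor, creates WBL_VictoryMenu and adds it to the viewport once a BP_GameInstance cast succeeds.
; It binds to the menu's button events: Play Again changes the game mode and Quit exits the game.
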(event Custom|OnVistoryMenu_PlayAgainClicked
  ;[1 1 1] Subscribe to Main Manu events
  (Utilities|ChangetheGameMode "NewEnumerator1"))

(event Custom|OnVictoryMenu_QuitClicked
  ;[1 1 1] Subscribe to Main Manu events
  (Utilities|QuittheGame))

(event EventBeginPlay
  (Utilities|FlowControl|Sequence
    (:then_0
      ;[1 1 1] Setup Input Mode
      (bind _asplayer_controller (Utilities|GetthePlayerController)
        (:%20%20
          (Input|SetInputModeUIOnly _asplayer_controller 0 "DoNotLock" false)
          (Variables|/Script/Engine.PlayerController|SetbShowMouseCursor _asplayer_controller true))))
    (:then_1
      ;[1 1 1] Create Main Menu
      (bind _returnvalue (UserInterface|CreateWidget "/Game/Widgets/WBL_VictoryMenu.WBL_VictoryMenu_C"))
      (Variables|Default|SetVictoryMenuRef _returnvalue)
      (Utilities|Casting|CastToBP_GameInstance (Game|GetGameInstance))
      (UserInterface|Viewport|AddtoViewport (Variables|Default|GetVictoryMenuRef) 0))
    (:then_2
      ;[1 1 1] Subscribe to Main Manu events
      (EventDispatchers|BindEventtoPlayAgainClicked (Variables|Default|GetVictoryMenuRef) (delegate Custom|OnVistoryMenu_PlayAgainClicked))
      (EventDispatchers|BindEventtoQuitClicked (Variables|Default|GetVictoryMenuRef) (delegate Custom|OnVictoryMenu_QuitClicked)))))

(fn ConstructionScript)