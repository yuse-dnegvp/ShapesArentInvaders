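; BP_Player is the player-controlled Blueprint that moves sideways along the world Y axis and fires on input.
; The MoveHorizontal axis adds movement input only while inside symmetric MovementBoundaries or when heading back toward center, using the sign of input times Y position.
; Pressing FireProjectile spawns an actor at the player's transform, though the spawned class is not shown.
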(event EventBeginPlay)

(event Collision|EventActorBeginOverlap
  (params (OtherActor :type Actor%20Object%20Reference)))

(event EventTick
  (params (DeltaSeconds :type Float%20%28single-precision%29)))

(event Input|ActionEvents|InputActionFireProjectile
  (params (Key :type Key%20Structure :default "None"))
  ;[1 1 1] Fire
  (:Pressed
    (CallFunction|FireProjectile)))

(event Input|AxisEvents|InputAxisMoveHorizontal
  (params (AxisValue :type Float%20%28single-precision%29))
  ;[1 1 1] Character Movement
  (CallFunction|MovePlayerRight AxisValue))

(fn ConstructionScript)

(fn MovePlayerRight
  (params (ScaleValue :type Float%20%28single-precision%29))
  (bind _returnvalue (Transformation|GetActorLocation))
  (bind _movementboundaries (Variables|Default|GetMovementBoundaries))
  (bind _y (Math|Vector|BreakVector _returnvalue))
  ;[1 1 1] Player Moving Inside (Towards) the Movement Boundaries?
  (if (or (< (* ScaleValue _y) 0.0) (Math|Float|InRange(Float) _y (* _movementboundaries -1.0) _movementboundaries))
    (Pawn|Input|AddMovementInput "0.000000,1.000000,0.000000" ScaleValue false)))

(fn FireProjectile
  (Game|SpawnActorfromClass "/Game/Blueprints/BP_Projectile.BP_Projectile_C" (Transformation|GetActorTransform) "Undefined" 0 0))