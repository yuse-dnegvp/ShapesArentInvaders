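; Platformer game mode that starts enemy spawning and keeps the score.
; On BeginPlay it tells its EnemyManager to spawn a row of enemies.
; OnEnemyHit and OnEnemyKilled events add their respective hit and kill rewards to Score.
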(event EventBeginPlay
  ;[1 1 1] Spawn Initial Enemies
  (Class|EnemyManager|SpawnEnemiesRow (Variables|Default|GetEnemyManager)))

(event EventTick
  (params (DeltaSeconds :type Float%20%28single-precision%29)))

(event EventOnEnemyHit
  ;[1 1 1] Enemy Hit Score Reward
  (Variables|Default|SetScore (+ (Variables|Default|GetHitReward) (Variables|Default|GetScore))))

(event EventOnEnemyKilled
  ;[1 1 1] Enemy Hit Killed Reward
  (Variables|Default|SetScore (+ (Variables|Default|GetKillReward) (Variables|Default|GetScore))))

(fn ConstructionScript)