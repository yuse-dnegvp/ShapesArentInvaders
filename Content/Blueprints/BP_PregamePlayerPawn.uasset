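; BP_PregamePlayerPawn is the player pawn for the pregame state, hosting the main menu.
; On BeginPlay it switches the player controller to UI-only input with a visible cursor and creates the main menu widget.
; It fills in the high score from the GameInstance's save reference.
; It binds the menu's Play click to a game mode change and its Quit click to quitting the game.
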(event Custom|OnMainMenu_PlayClicked
  ;[1 1 1] Subscribe to Main Manu events
  (Utilities|ChangetheGameMode "NewEnumerator1"))

(event Custom|OnMainMenu_QuitClicked
  ;[1 1 1] Subscribe to Main Manu events
  (Utilities|QuittheGame))

(event EventBeginPlay
  (Utilities|FlowControl|Sequence
    (:then_0
      ;[1 1 1] Setup UI Mode
      (bind _asplayer_controller (Utilities|GetthePlayerController)
        (:%20%20
          (Input|SetInputModeUIOnly _asplayer_controller 0 "DoNotLock" false)
          (Variables|/Script/Engine.PlayerController|SetbShowMouseCursor _asplayer_controller true))))
    (:then_1
      ;[1 1 1] Create Main Menu
      (bind _returnvalue (UserInterface|CreateWidget "/Game/Widgets/WBL_MainMenu.WBL_MainMenu_C"))
      (Variables|Default|SetMainMenuRef _returnvalue)
      (bind _asbp_game_instance (Utilities|Casting|CastToBP_GameInstance (Game|GetGameInstance)))
      (Default|SetHighScore (Variables|Default|GetMainMenuRef) (Variables|/Game/Blueprints/BP_SaveHighScore.BP_SaveHighScore_C|GetHighScore (Variables|/Game/Blueprints/BP_GameInstance.BP_GameInstance_C|GetSaveHighScoreRef _asbp_game_instance)))
      (UserInterface|Viewport|AddtoViewport (Variables|Default|GetMainMenuRef) 0))
    (:then_2
      ;[1 1 1] Subscribe to Main Manu events
      (EventDispatchers|BindEventtoPlayClicked (Variables|Default|GetMainMenuRef) (delegate Custom|OnMainMenu_PlayClicked))
      (EventDispatchers|BindEventtoQuitClicked (Variables|Default|GetMainMenuRef) (delegate Custom|OnMainMenu_QuitClicked)))))

(fn ConstructionScript)